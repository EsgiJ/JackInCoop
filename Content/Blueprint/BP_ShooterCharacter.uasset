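; BP_ShooterCharacter is a shooter character Blueprint that sets up the local player's HUD and provides a movement input helper.
; On BeginPlay, only the locally controlled instance creates crosshair, health indicator, health bar and ammo clip widgets and adds them to the viewport.
; ClampInputScale normalizes 2D input and snaps its magnitude to a run or walk scale, depending on whether it exceeds the run threshold.
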(event `self.ReceiveBeginPlay`
  (if (`self.IsLocallyControlled`)
    (`|ExecutionSequence`
      (:`then_0`
        ;[1 1 1] HUD | Widgets
        (bind _returnvalue (`|CreateWidget` "/Game/UI/WBP_Crosshair.WBP_Crosshair_C"))
        (`UserWidget.AddToViewport` _returnvalue 0))
      (:`then_1`
        (bind _returnvalue_2 (`|CreateWidget` "/Game/UI/WBP_HealthIndicator.WBP_HealthIndicator_C"))
        (`UserWidget.AddToViewport` _returnvalue_2 0))
      (:`then_2`
        (bind _returnvalue_3 (`|CreateWidget` "/Game/UI/WBP_HealthBar.WBP_HealthBar_C"))
        (`UserWidget.AddToViewport` _returnvalue_3 0))
      (:`then_3`
        (bind _returnvalue_4 (`|CreateWidget` "/Game/UI/WBP_AmmoClip.WBP_AmmoClip_C"))
        (`UserWidget.AddToViewport` _returnvalue_4 0)))))

(fn `ClampInputScale`
  (params (InputScale :type "Vector2D Structure"))
  (returns (ReturnValue :type "Vector2D Structure"))
  (if (> (`KismetMathLibrary.VSize2D` InputScale) (`self.RunScaleThreshold`))
    (return (* (`KismetMathLibrary.Normal2D` InputScale) (`self.RunScale`)))
    (else
      (return (* (`KismetMathLibrary.Normal2D` InputScale) (`self.WalkScale`))))))

(fn `UserConstructionScript`)