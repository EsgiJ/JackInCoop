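; Test game mode that rewards players for kills and spawns tracker bots.
; On actor killed, it adds score to the killer's SPlayerState when the victim is a pawn not controlled by a player, then prints the total.
; SpawnNewBot runs an EQS query, picking randomly from the best 25%, and spawns BP_TrackerBot at the returned location, adjusting for collision or skipping if blocked.
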(event `self.ReceiveBeginPlay`
  (add `self.OnActorKilled` (delegate `OnActorKilled_Event`)))

(event `OnActorKilled_Event` :!signature `self.OnActorKilled`
  (params (VictimActor :type "Actor Object Reference") (KillerActor :type "Actor Object Reference") (KillerController :type "Controller Object Reference"))
  ;[1 1 1] Don't reward friendly fire
  (bind _aspawn (cast `Pawn` VictimActor))
  (if (not (`Pawn.IsPlayerControlled` _aspawn))
    ;[1 1 1] Add Score for killing enemy
    (bind _assplayer_state (cast `SPlayerState` (`Pawn.PlayerState` (`Controller.K2_GetPawn` KillerController))))
    (`SPlayerState.AddScore` _assplayer_state 5.0)
    (`KismetSystemLibrary.PrintString` (`KismetStringLibrary.Conv_DoubleToString` (`PlayerState.Score` _assplayer_state)) true true (struct :`R` 0.019536 :`B` 1.0 :`A` 1.0) 5.0)))

(event `self.SpawnNewBot`
  (bind _returnvalue (`EnvQueryManager.RunEQSQuery` "/Game/Blueprint/EQS_FindSpawnLocation.EQS_FindSpawnLocation" self "RandomBest25Pct"))
  (add `EnvQueryInstanceBlueprintWrapper.OnQueryFinishedEvent` _returnvalue (delegate `OnQueryFinishedEvent_Event`)))

(event `OnQueryFinishedEvent_Event`
  (params (QueryInstance :type "EnvQueryInstanceBlueprintWrapper Object Reference") (QueryStatus :type "EEnvQueryStatus Enum" :default "Processing"))
  (bind _resultlocations (`EnvQueryInstanceBlueprintWrapper.GetQueryResultsAsLocations` QueryInstance))
  (switch `EEnvQueryStatus` QueryStatus
    (:`Success`
      (for _array_element _resultlocations
        (`|SpawnActorFromClass` "/Game/TrackerBot/BP_TrackerBot.BP_TrackerBot_C" (`KismetMathLibrary.MakeTransform` _array_element) "AdjustIfPossibleButDontSpawnIfColliding" "MultiplyWithRoot" null null)))))

(fn `UserConstructionScript`)