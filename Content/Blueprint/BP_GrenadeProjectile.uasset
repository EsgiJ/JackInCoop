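; Grenade projectile actor that explodes on impact or after a one-second fuse, then destroys itself.
; Both BeginPlay's delay and the Hit event call Explode, which applies radial damage around the actor using DamageRadius, credited to the instigator's controller.
; Explode also spawns a scaled-up explosion particle and plays the explosion sound, which is placed at world origin instead of the grenade's location.
; A debug sphere draw remains in the graph but never runs.
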(event `self.ReceiveBeginPlay`
  (`KismetSystemLibrary.Delay` 1.0)
  (`self.Explode`)
  (`self.K2_DestroyActor`))

(event `Explode`
  (bind _returnvalue (`self.K2_GetActorLocation`))
  (`GameplayStatics.ApplyRadialDamage` :`BaseDamage` 60.0 :`Origin` _returnvalue :`DamageRadius` (`self.Damage Radius`) :`DamageCauser` self :`InstigatedByController` (`self.GetInstigatorController`))
  (`GameplayStatics.SpawnEmitterAtLocation` "/Game/WeaponEffects/Explosion/P_Explosion.P_Explosion" _returnvalue (struct) (2.0 2.0 2.0))
  (`GameplayStatics.PlaySoundAtLocation` "/Game/Sound/GrenadeLauncherSounds/GrenadeLauncher_ExplosionSound.GrenadeLauncher_ExplosionSound" (0.0 0.0 0.0) (struct) 1.0 1.0 0.0 null null null null))

(event `self.ReceiveHit`
  (params (MyComp :type "PrimitiveComponent Object Reference") (Other :type "Actor Object Reference") (OtherComp :type "PrimitiveComponent Object Reference") (bSelfMoved :type Boolean) (HitLocation :type "Vector Structure") (HitNormal :type "Vector Structure") (NormalImpulse :type "Vector Structure") (Hit :type "HitResult Structure (by ref)"))
  (`self.Explode`)
  (`self.K2_DestroyActor`))

(fn `UserConstructionScript`)