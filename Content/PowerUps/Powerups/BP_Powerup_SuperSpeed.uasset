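; Super speed power-up that doubles the walk speed of the player who activates it until it expires.
; On activation it stores that player and sets their Character Movement MaxWalkSpeed to twice the current GetMaxSpeed.
; On expiry it sets MaxWalkSpeed to half the then-current GetMaxSpeed if the player is still valid, rather than restoring a saved value, then calls the parent's expiry logic.
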(event `self.OnActivated`
  (params (ActivateFor :type "Actor Object Reference"))
  (bind _returnvalue (`self.GetComponentByClass` ActivateFor "/Script/Engine.CharacterMovementComponent"))
  (set `self.ActivateForPlayer` ActivateFor)
  (set `CharacterMovementComponent.MaxWalkSpeed` (* (`MovementComponent.GetMaxSpeed` _returnvalue) 2.0) _returnvalue))

(event `self.OnExpired`
  (bind _activateforplayer (`self.ActivateForPlayer`))
  (bind _returnvalue (`self.GetComponentByClass` _activateforplayer "/Script/Engine.CharacterMovementComponent"))
  (`/Engine/EditorBlueprintResources/StandardMacros.IsValid` _activateforplayer
    (:`Is Valid`
      (set `CharacterMovementComponent.MaxWalkSpeed` (/ (`MovementComponent.GetMaxSpeed` _returnvalue) 2.0) _returnvalue))
    (:`Is Not Valid`
      _))
  (`parent.OnExpired`))

(fn `UserConstructionScript`)