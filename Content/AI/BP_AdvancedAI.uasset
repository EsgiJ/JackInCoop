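; BP_AdvancedAI is an AI character that runs the BT_AdvancedAI behavior tree on its AI controller at BeginPlay.
; Any health change reported by its HealthComponent plays a random montage from HitReactions.
; Montages are broadcast through a PlayMontageOnServer event that forwards to PlayMontageOnClient, which plays the animation.
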(event `self.ReceiveBeginPlay`
  (`AIController.RunBehaviorTree` (`AIBlueprintHelperLibrary.GetAIController` self) "/Game/AI/BT_AdvancedAI.BT_AdvancedAI"))

(event `self.HealthComponent.OnHealthChanged`
  (params (HealthComponent :type "HealthComponent Object Reference") (Health :type "Float (single-precision)") (HealthDelta :type "Float (single-precision)") (DamageType :type "DamageType Object Reference") (InstigatedBy :type "Controller Object Reference") (DamageCauser :type "Actor Object Reference"))
  ;[1 1 1] Hit Reaction Anim Montages
  (`self.Play Montage On Server` (`KismetArrayLibrary.Array_Random` (`self.HitReactions`))))

(event `Play Montage On Server`
  (params (AnimMontage :type "AnimMontage Object Reference"))
  ;[1 1 1] Broadcast Anim Montage
  (`self.Play Montage On Client` AnimMontage))

(event `Play Montage On Client`
  (params (AnimMontage :type "AnimMontage Object Reference"))
  ;[1 1 1] Broadcast Anim Montage
  (`self.PlayAnimMontage` AnimMontage))

(fn `UserConstructionScript`)