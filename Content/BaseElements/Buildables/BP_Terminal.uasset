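; BP_Terminal is a buildable terminal Blueprint that labels its interaction prompt widget.
; On BeginPlay, after the parent logic, it casts the Widget component's user widget to WBP_Interact and sets its InteractText to "Interact".
; The construction script only calls its parent, and this file has no logic for what happens upon interaction.
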(event `self.ReceiveBeginPlay`
  (`parent.ReceiveBeginPlay`)
  (bind _aswbp_interact (cast `/Game/UI/WBP_Interact` (`WidgetComponent.GetUserWidgetObject` (`self.Widget`))))
  (set `/Game/UI/WBP_Interact.InteractText` "Interact" _aswbp_interact))

(fn `UserConstructionScript`
  (`parent.UserConstructionScript`))