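; Interactable pistol ammo crate that grants ammo to a shooter character who uses it.
; On begin play it sets the interact widget's text to a pickup prompt, and the interaction radius overlap events show and hide that widget.
; OnInteract casts the interactor to the shooter character and calls GrantAmmo on its primary weapon only when the current weapon type is pistol.
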(event `self.ReceiveBeginPlay`
  (`parent.ReceiveBeginPlay`)
  (bind _aswbp_interact (cast `/Game/UI/WBP_Interact` (`WidgetComponent.GetUserWidgetObject` (`self.Widget`))))
  (set `/Game/UI/WBP_Interact.InteractText` "Pick Up Ammo" _aswbp_interact))

(event `self.OnInteract`
  (params (Interactor :type "ShooterCharacter Object Reference"))
  (bind _asbp_shooter_character (cast `/Game/Blueprint/BP_ShooterCharacter` Interactor))
  (if (`|EnumEquality` (`ShooterCharacter.CurrentWeaponType` _asbp_shooter_character) "Pistol")
    (`ShooterWeapon.GrantAmmo` (`ShooterCharacter.PrimaryWeapon` _asbp_shooter_character))))

(event `self.InteractibleRadius.OnComponentBeginOverlap`
  (params (OverlappedComponent :type "PrimitiveComponent Object Reference") (OtherActor :type "Actor Object Reference") (OtherComp :type "PrimitiveComponent Object Reference") (OtherBodyIndex :type Integer) (bFromSweep :type Boolean) (SweepResult :type "HitResult Structure (by ref)"))
  (`SceneComponent.SetVisibility` (`self.Widget`) true true))

(event `self.InteractibleRadius.OnComponentEndOverlap`
  (params (OverlappedComponent :type "PrimitiveComponent Object Reference") (OtherActor :type "Actor Object Reference") (OtherComp :type "PrimitiveComponent Object Reference") (OtherBodyIndex :type Integer))
  (`SceneComponent.SetVisibility` (`self.Widget`) false true))

(fn `UserConstructionScript`
  (`parent.UserConstructionScript`))